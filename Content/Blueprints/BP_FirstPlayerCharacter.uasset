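; First-person player character with double-jump and wall-running movement.
; A DoN counter, reset on landing or wall-capsule overlap, limits upward launches for the double jump.
; Touching a "Runable" actor while falling starts a timeline that, while Space is held, removes gravity, locks vertical movement with a plane constraint and pushes along the camera direction captured on contact.
; Releasing Space or leaving the wall restores normal movement.
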(event `self.ReceiveBeginPlay`
  ;[1 1 1] BeginPlay
  (`MovementComponent.SetPlaneConstraintEnabled` (`self.CharacterMovement`) true))

(event `self.OnLanded`
  (params (Hit :type "HitResult Structure (by ref)"))
  ;[1 1 1] Double Jump
  (bind _counter (`/Engine/EditorBlueprintResources/StandardMacros.Do N` 2 :!via `Reset` :!label _label)
    (:`Exit`
      (switch `int` _counter
        (:`1`
          _)
        (:`2`
          _))
      (`self.LaunchCharacter` (0.0 0.0 420.0) false true))))

(event `InputAction|Jump`
  (params (Key :type "Key Structure"))
  ;[1 1 1] Double Jump
  (:`Released`
    (`self.StopJumping`)))

(event `self.WallRunningCapsule.OnComponentBeginOverlap`
  (params (OverlappedComponent :type "PrimitiveComponent Object Reference") (OtherActor :type "Actor Object Reference") (OtherComp :type "PrimitiveComponent Object Reference") (OtherBodyIndex :type Integer) (bFromSweep :type Boolean) (SweepResult :type "HitResult Structure (by ref)"))
  (bind _charactermovement (`self.CharacterMovement`))
  (bind _charactermovement_2 (`self.CharacterMovement`))
  (`|ExecutionSequence`
    (:`then_0`
      (goto _label :!via `Reset`))
    (:`then_1`
      (set `self.PlayerDirection` (`SceneComponent.GetForwardVector` (`self.Camera`)))
      (if (and (`self.ActorHasTag` OtherActor "Runable") (`NavMovementComponent.IsFalling` (`self.CharacterMovement`)))
        (set `self.OnWall` true)
        (`Timeline|WallRun` :!label _label_2
          (:`Update`
            (if (> (`PlayerController.GetInputKeyTimeDown` (`GameplayStatics.GetPlayerController` 0) "SpaceBar") 0.0)
              (if (`self.OnWall`)
                (set `CharacterMovementComponent.GravityScale` 0.0 _charactermovement_2)
                (`MovementComponent.SetPlaneConstraintNormal` _charactermovement_2 (0.0 0.0 1.0))
                (`CharacterMovementComponent.AddForce` _charactermovement_2 (* (`self.PlayerDirection`) 20000.0))
                (else
                  (set `CharacterMovementComponent.GravityScale` 1.0 _charactermovement :!label _label_3)
                  (`MovementComponent.SetPlaneConstraintNormal` _charactermovement (0.0 0.0 0.0))
                  (set `self.OnWall` false)))
              (else
                (goto _label_3)))))))))

(event `self.WallRunningCapsule.OnComponentEndOverlap`
  (params (OverlappedComponent :type "PrimitiveComponent Object Reference") (OtherActor :type "Actor Object Reference") (OtherComp :type "PrimitiveComponent Object Reference") (OtherBodyIndex :type Integer))
  (`|ExecutionSequence`
    (:`then_0`
      (goto _label_2 :!via `Stop`))
    (:`then_1`
      (if (`self.ActorHasTag` OtherActor "Runable")
        (goto _label_3)))))

(fn `UserConstructionScript`)